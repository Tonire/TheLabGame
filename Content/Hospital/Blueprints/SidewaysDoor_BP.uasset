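; SidewaysDoor_BP is a double door in the Hospital content whose left and right panels move apart or along set paths when opened.
; OpenDoor plays the MoverDoors timeline from the start, feeding its two tracks into the relative locations of LeftDoor and RightDoor.
; CloseDoor is empty, and an unconnected VInterpTo chain that moves each panel toward a sphere marker's X position never runs.
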(event `OpenDoor`
  (bind (_direction _leftdoor _rightdoor) (`Timeline|MoverDoors` :!via `PlayFromStart`)
    (:`Update`
      (`SceneComponent.K2_SetRelativeLocation` (`self.LeftDoor`) _leftdoor false false)
      (`SceneComponent.K2_SetRelativeLocation` (`self.RightDoor`) _rightdoor false false))))

(event `CloseDoor`)

(fn `UserConstructionScript`)