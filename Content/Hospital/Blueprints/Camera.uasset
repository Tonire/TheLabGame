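; Security camera that detects the VR player (MotionControllerPawn) with a view cone and light, printing "MUERTO" after two seconds of tracking.
; Each tick a forward trace sets the laser's end, and lock-on compares player distance to laser length as an approximate occlusion check.
; While locked with the player in the cone, it smoothly follows them; otherwise it plays a looping rotation timeline or returns to its initial rotation.
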(event `self.ReceiveTick`
  (params (DeltaSeconds :type "Float (single-precision)"))
  (`self.UpdateLaser`)
  (`self.CheckAndLockTarget`)
  (if (`self.LockedOnTarget`)
    (if (`self.TouchingCone`)
      (`self.MoveCameraTowardsPawn`)
      (bind _output_get (set `self.TimeTarget` (+ DeltaSeconds (`self.TimeTarget`))))
      (if (>= _output_get 2.0)
        (`KismetSystemLibrary.PrintString` "MUERTO"))
      (else
        (if (`self.Animated`) :!label _label
          (bind (_direction _camerarotation) (`Timeline|CameraRotation` :!label _label_2)
            (:`Update`
              (if (`self.TouchingCone`)
                (goto _label_2 :!via `Stop`)
                (else
                  (`self.RotateCamera` _camerarotation)
                  (set `self.TimeTarget` 0.0 :!label _label_3)))))
          (else
            (`self.PointCameraToInitialRotation`)
            (goto _label_3)))))
    (else
      (goto _label))))

(event `self.Cone.OnComponentBeginOverlap`
  (params (OverlappedComponent :type "PrimitiveComponent Object Reference") (OtherActor :type "Actor Object Reference") (OtherComp :type "PrimitiveComponent Object Reference") (OtherBodyIndex :type Integer) (bFromSweep :type Boolean) (SweepResult :type "HitResult Structure (by ref)"))
  (`/Engine/EditorBlueprintResources/StandardMacros.IsValid` OtherActor
    (:`Is Valid`
      (bind _asmotion_controller_pawn (cast `/Game/VirtualRealityBP/Blueprints/MotionControllerPawn` OtherActor))
      (set `self.PlayerPawn` _asmotion_controller_pawn)
      (set `self.LockedOnTarget` true)
      (set `self.TouchingCone` true)
      (`self.ChangeLightColour` (struct :`R` 0.895 :`G` 0.763434 :`A` 1.0)))))

(event `self.Cone.OnComponentEndOverlap`
  (params (OverlappedComponent :type "PrimitiveComponent Object Reference") (OtherActor :type "Actor Object Reference") (OtherComp :type "PrimitiveComponent Object Reference") (OtherBodyIndex :type Integer))
  (`/Engine/EditorBlueprintResources/StandardMacros.IsValid` OtherActor
    (:`Is Valid`
      (cast `/Game/VirtualRealityBP/Blueprints/MotionControllerPawn` OtherActor)
      (set `self.PlayerPawn` null)
      (set `self.TargetPoint` (0.0 0.0 0.0))
      (set `self.LockedOnTarget` false)
      (set `self.TouchingCone` false)
      (`self.ChangeLightColour` (`self.LightColour`)))))

(fn `ChangeLightColour`
  (params (NewColour :type "LinearColor Structure"))
  (`LightComponent.SetLightColor` (`self.Light`) NewColour true))

(fn `CheckAndLockTarget`
  (bind _returnvalue (`SceneComponent.K2_GetComponentLocation` (`self.LaserStartPoint`)))
  ;[1 1 1] Nos aseguramos de que el jugador es visible por la camara (no está detrás de ningún objeto)
  (if (<= (`KismetMathLibrary.VSizeSquared` (- (`self.K2_GetActorLocation` (`GameplayStatics.GetPlayerPawn` 0)) _returnvalue)) (`KismetMathLibrary.VSizeSquared` (- (`self.LaserEndPoint`) _returnvalue)))
    ;[1 1 1] Sí está al alcance de la camara
    (set `self.LockedOnTarget` true)
    (bind _asmotion_controller_pawn (cast `/Game/VirtualRealityBP/Blueprints/MotionControllerPawn` (`GameplayStatics.GetPlayerPawn` 0)))
    (set `self.PlayerPawn` _asmotion_controller_pawn)
    (else
      ;[1 1 1] No está al alcance de la camara
      (set `self.LockedOnTarget` false)
      (set `self.PlayerPawn` null))))

(fn `MoveCameraTowardsPawn`
  ;[1 1 1] Apuntamos la cámara al jugador
  (if (`self.LockedOnTarget`)
    (bind _output_get (set `self.TargetPoint` (`self.K2_GetActorLocation` (`self.PlayerPawn`))))
    (bind (_returnvalue_roll _returnvalue_pitch _returnvalue_yaw) (`KismetMathLibrary.BreakRotator` (`KismetMathLibrary.FindLookAtRotation` (`SceneComponent.K2_GetComponentLocation` (`self.CameraBody`)) _output_get)))
    ;[1 1 1] Rotamos
    (`SceneComponent.K2_SetRelativeRotation` (`self.CameraBody`) (`KismetMathLibrary.RInterpTo` (`SceneComponent.RelativeRotation` (`self.CameraBody`)) (`KismetMathLibrary.MakeRotator` (* _returnvalue_pitch -1.0) _returnvalue_roll (+ _returnvalue_yaw -90.0)) (`GameplayStatics.GetWorldDeltaSeconds`) 5.0) false false)))

(fn `PointCameraToInitialRotation`
  (bind _camerabody (`self.CameraBody`))
  (`SceneComponent.K2_SetRelativeRotation` _camerabody (`KismetMathLibrary.RInterpTo` (`SceneComponent.RelativeRotation` _camerabody) (`self.InitialRotation`) (`GameplayStatics.GetWorldDeltaSeconds`) 5.0) false false))

(fn `RotateCamera`
  (params (NewRotation :type "Vector Structure"))
  (bind _returnvalue (`GameplayStatics.GetWorldDeltaSeconds`))
  (bind _camerabody (`self.CameraBody`))
  (bind (_relativerotation_roll _relativerotation_pitch _relativerotation_yaw) (`KismetMathLibrary.BreakRotator` (`SceneComponent.RelativeRotation` _camerabody)))
  (`SceneComponent.K2_SetRelativeRotation` _camerabody (`KismetMathLibrary.MakeRotator` (`KismetMathLibrary.FInterpTo` _relativerotation_roll NewRotation_X _returnvalue 5.0) (`KismetMathLibrary.FInterpTo` _relativerotation_pitch NewRotation_Y _returnvalue 5.0) (`KismetMathLibrary.FInterpTo` _relativerotation_yaw NewRotation_Z _returnvalue 5.0)) false false))

(fn `UpdateLaser`
  (bind _laserstartpoint (`self.LaserStartPoint`))
  (bind (_returnvalue_x _returnvalue_y _returnvalue_z) (`KismetMathLibrary.BreakVector` (+ (`SceneComponent.K2_GetComponentLocation` _laserstartpoint) (* (`SceneComponent.GetForwardVector` _laserstartpoint) (`self.ViewDistance`)))))
  (bind _output_get (set `self.LaserEndPoint` (`KismetMathLibrary.MakeVector` _returnvalue_x _returnvalue_y (- _returnvalue_z 10.0))))
  (bind (_outhit _returnvalue) (`KismetSystemLibrary.LineTraceSingle` (`SceneComponent.K2_GetComponentLocation` (`self.LaserStartPoint`)) _output_get "TraceTypeQuery1" false (`|MakeArray` (`GameplayStatics.GetPlayerPawn` 0) :!type "Actor Object Reference")))
  (if _returnvalue
    (bind _output_get_2 (set `self.LaserEndPoint` (`.Location` (`GameplayStatics.BreakHitResult` _outhit)))))
  (`ParticleSystemComponent.SetBeamEndPoint` (`self.LaserBeam`) 0 (`KismetMathLibrary.MakeVector` (.x _output_get_2) (.y _output_get_2) (- (.z _output_get_2) 10.0))))

(fn `UserConstructionScript`
  (bind _light (`self.Light`))
  (`self.PointCameraToInitialRotation`)
  (`SceneComponent.K2_AttachToComponent` (`self.CameraBody`) (`self.CameraStand`) "Base" "KeepRelative" "KeepWorld" "KeepRelative" true)
  (`LightComponent.SetLightColor` _light (`self.LightColour`) true)
  (`LightComponent.SetIntensity` _light (`self.LightIntensity`))
  (`self.UpdateLaser`)
  (`TimelineComponent.SetLooping` (`self.CameraRotation`) true))