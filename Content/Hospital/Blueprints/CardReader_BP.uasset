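; VR card reader that opens its linked door and signals level 1 completion when the matching keycard is used.
; Box overlap releases held items from the motion controllers, eases the card toward LittleSphere and tints the reader blue.
; Tick locks the card's X/Y and rotation to that sphere, keeping its current Z.
; LittleSphere contact arms opening; ActivationSphere then checks the card name and turns the reader green.
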(event `self.ReceiveTick`
  (params (DeltaSeconds :type "Float (single-precision)"))
  (bind _returnvalue (`GameplayStatics.GetWorldDeltaSeconds`))
  (bind _littlesphere (`self.LittleSphere`))
  (bind (_returnvalue_x _returnvalue_y) (`KismetMathLibrary.BreakVector` (`SceneComponent.K2_GetComponentLocation` _littlesphere)))
  (bind _staticmeshcomponent (`StaticMeshActor.StaticMeshComponent` (`self.KeyCardBP`)))
  (bind _returnvalue_2 (`SceneComponent.K2_GetComponentLocation` _staticmeshcomponent))
  (`/Engine/EditorBlueprintResources/StandardMacros.IsValid` (`self.KeyCardBP`)
    (:`Is Valid`
      (`SceneComponent.K2_SetWorldLocationAndRotation` _staticmeshcomponent (`KismetMathLibrary.VInterpTo` _returnvalue_2 (`KismetMathLibrary.MakeVector` _returnvalue_x _returnvalue_y (.z _returnvalue_2)) _returnvalue 200.0) (`KismetMathLibrary.Conv_VectorToRotator` (`KismetMathLibrary.VInterpTo` (`KismetMathLibrary.Conv_RotatorToVector` (`SceneComponent.K2_GetComponentRotation` _staticmeshcomponent)) (`KismetMathLibrary.Conv_RotatorToVector` (`SceneComponent.K2_GetComponentRotation` _littlesphere)) _returnvalue 200.0)) false false))))

(event `self.Box.OnComponentBeginOverlap`
  (params (OverlappedComponent :type "PrimitiveComponent Object Reference") (OtherActor :type "Actor Object Reference") (OtherComp :type "PrimitiveComponent Object Reference") (OtherBodyIndex :type Integer) (bFromSweep :type Boolean) (SweepResult :type "HitResult Structure (by ref)"))
  (bind _askey_card_bp (cast `/Game/Hospital/Blueprints/KeyCard_BP` OtherActor))
  (set `self.KeyCardBP` _askey_card_bp)
  (if (`self.ShouldUseCard`)
    (set `self.ShouldUseCard` false)
    (`self.UseCard`)))

(event `self.Box.OnComponentEndOverlap`
  (params (OverlappedComponent :type "PrimitiveComponent Object Reference") (OtherActor :type "Actor Object Reference") (OtherComp :type "PrimitiveComponent Object Reference") (OtherBodyIndex :type Integer))
  (cast `/Game/Hospital/Blueprints/KeyCard_BP` OtherActor)
  (set `self.KeyCardBP` null)
  (set `self.ShouldUseCard` true))

(event `self.ActivationSphere.OnComponentBeginOverlap`
  (params (OverlappedComponent :type "PrimitiveComponent Object Reference") (OtherActor :type "Actor Object Reference") (OtherComp :type "PrimitiveComponent Object Reference") (OtherBodyIndex :type Integer) (bFromSweep :type Boolean) (SweepResult :type "HitResult Structure (by ref)"))
  (bind _askey_card_bp (cast `/Game/Hospital/Blueprints/KeyCard_BP` OtherActor))
  (if (`KismetStringLibrary.EqualEqual_StrStr` (`/Game/Hospital/Blueprints/KeyCard_BP.CardName` _askey_card_bp) (`self.Card`))
    (if (`self.CanOpen`)
      (`self.OpenAndChangeToGreen`))))

(event `MoveCardSmoothly`
  (bind _returnvalue (`GameplayStatics.GetWorldDeltaSeconds`))
  (bind _littlesphere (`self.LittleSphere`))
  (bind _staticmeshcomponent (`StaticMeshActor.StaticMeshComponent` (`self.KeyCardBP`)))
  (`/Engine/EditorBlueprintResources/StandardMacros.IsValid` (`self.KeyCardBP`)
    (:`Is Valid`
      (`Timeline|Timeline_0`
        (:`Update`
          (`/Engine/EditorBlueprintResources/StandardMacros.IsValid` (`self.KeyCardBP`)
            (:`Is Valid`
              (`SceneComponent.K2_SetWorldLocationAndRotation` _staticmeshcomponent (`KismetMathLibrary.VInterpTo` (`SceneComponent.K2_GetComponentLocation` _staticmeshcomponent) (`SceneComponent.K2_GetComponentLocation` _littlesphere) _returnvalue 15.0) (`KismetMathLibrary.Conv_VectorToRotator` (`KismetMathLibrary.VInterpTo` (`KismetMathLibrary.Conv_RotatorToVector` (`SceneComponent.K2_GetComponentRotation` _staticmeshcomponent)) (`KismetMathLibrary.Conv_RotatorToVector` (`SceneComponent.K2_GetComponentRotation` _littlesphere)) _returnvalue 15.0)) false false))))))))

(event `self.LittleSphere.OnComponentBeginOverlap`
  (params (OverlappedComponent :type "PrimitiveComponent Object Reference") (OtherActor :type "Actor Object Reference") (OtherComp :type "PrimitiveComponent Object Reference") (OtherBodyIndex :type Integer) (bFromSweep :type Boolean) (SweepResult :type "HitResult Structure (by ref)"))
  (cast `/Game/Hospital/Blueprints/KeyCard_BP` OtherActor)
  (set `self.CanOpen` true))

(fn `OpenAndChangeToGreen`
  (bind _staticmesh (`self.StaticMesh`))
  (bind _returnvalue (`PrimitiveComponent.CreateDynamicMaterialInstance` _staticmesh 1 (`PrimitiveComponent.GetMaterial` _staticmesh 1)))
  (`MaterialInstanceDynamic.SetVectorParameterValue` _returnvalue "Colour" (struct :`R` 0.011976 :`G` 1.0 :`A` 1.0))
  (if (not (`self.Open`))
    (`/Game/Hospital/Blueprints/SidewaysDoor_BP.OpenDoor` (`self.Door`))
    (set `self.Open` true)
    (`self.Level1Completed`)))

(fn `UseCard`
  (bind _staticmesh (`self.StaticMesh`))
  (bind _asmotion_controller_pawn (cast `/Game/VirtualRealityBP/Blueprints/MotionControllerPawn` (`GameplayStatics.GetPlayerPawn` 0)))
  (`|ExecutionSequence`
    (:`then_0`
      (bind _rightcontroller (`/Game/VirtualRealityBP/Blueprints/MotionControllerPawn.RightController` _asmotion_controller_pawn))
      (if (`KismetSystemLibrary.IsValid` (`/Game/VirtualRealityBP/Blueprints/BP_MotionController.AttachedActor` _rightcontroller))
        (`/Game/VirtualRealityBP/Blueprints/BP_MotionController.ReleaseActor` _rightcontroller)
        (`self.MoveCardSmoothly` :!label _label)
        (if (not (`self.Open`))
          (bind _returnvalue (`PrimitiveComponent.CreateDynamicMaterialInstance` _staticmesh 1 (`PrimitiveComponent.GetMaterial` _staticmesh 1)))
          (`MaterialInstanceDynamic.SetVectorParameterValue` _returnvalue "Colour" (struct :`G` 0.038633 :`B` 0.58 :`A` 1.0)))))
    (:`then_1`
      (bind _leftcontroller (`/Game/VirtualRealityBP/Blueprints/MotionControllerPawn.LeftController` _asmotion_controller_pawn))
      (if (`KismetSystemLibrary.IsValid` (`/Game/VirtualRealityBP/Blueprints/BP_MotionController.AttachedActor` _leftcontroller))
        (`/Game/VirtualRealityBP/Blueprints/BP_MotionController.ReleaseActor` _leftcontroller)
        (goto _label)))))

(fn `UserConstructionScript`)