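; KeyPad_BP is a hospital keypad actor that records key presses made with VR motion controllers.
; When a BP_MotionController overlaps the "1" component, the only key wired up, it calls NewKeyPressed with 1.
; That function stores up to four presses as strings in Keys, tracked by KeyCounter, then runs an empty loop over them.
; No code checking or unlock response is implemented.
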(event `self.1.OnComponentBeginOverlap`
  (params (OverlappedComponent :type "PrimitiveComponent Object Reference") (OtherActor :type "Actor Object Reference") (OtherComp :type "PrimitiveComponent Object Reference") (OtherBodyIndex :type Integer) (bFromSweep :type Boolean) (SweepResult :type "HitResult Structure (by ref)"))
  (cast `/Game/VirtualRealityBP/Blueprints/BP_MotionController` OtherActor)
  (`self.newKeyPressed` 1))

(fn `newKeyPressed`
  (params (Key :type Integer))
  (bind _keys (`self.Keys`))
  (if (< (`self.KeyCounter`) 4)
    (`/Engine/EditorBlueprintResources/StandardMacros.IncrementInt` (`self.KeyCounter`)
      (:`  `
        (`KismetArrayLibrary.Array_Add` _keys (`KismetStringLibrary.Conv_IntToString` Key))
        (for _ _keys
          _)))))

(fn `UserConstructionScript`)