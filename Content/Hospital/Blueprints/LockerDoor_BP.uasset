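; LockerDoor_BP is a locker door that a VR motion controller can grab and move through physics.
; Pickup, called by BP_MotionController, stores the controller and grabs the mesh with a PhysicsHandle at the hand's location.
; Tick drives the handle's target to the controller, so the door is pulled physically instead of being attached.
; Drop clears the controller, re-enables physics simulation, detaches the actor and releases the handle.
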(event `self.ReceiveTick`
  (params (DeltaSeconds :type "Float (single-precision)"))
  (bind _controller (`self.Controller`))
  (if (`KismetSystemLibrary.IsValid` _controller)
    (`PhysicsHandleComponent.SetTargetLocation` (`self.PhysicsHandle`) (`SceneComponent.K2_GetComponentLocation` _controller))))

(event `/Game/VirtualRealityBP/Blueprints/PickupActorInterface.Pickup`
  (params (AttachTo :type "SceneComponent Object Reference"))
  (bind _output_get (set `self.Controller` AttachTo))
  (`PhysicsHandleComponent.GrabComponentAtLocation` (`self.PhysicsHandle`) (`self.StaticMeshComponent`) "None" (`SceneComponent.K2_GetComponentLocation` _output_get)))

(event `/Game/VirtualRealityBP/Blueprints/PickupActorInterface.Drop`
  (set `self.Controller` null)
  (`PrimitiveComponent.SetSimulatePhysics` (`self.StaticMeshComponent`) true)
  (`self.K2_DetachFromActor` "KeepWorld" "KeepWorld" "KeepWorld")
  (`PhysicsHandleComponent.ReleaseComponent` (`self.PhysicsHandle`)))

(fn `UserConstructionScript`)